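; BP_Weapon is a self-pickup actor that gives the player character a random weapon on overlap.
; When a BP_MyCharacter overlaps its mesh, it compares randomly indexed DT_Weapon row names against Pistol and Rifle, falling back to Launcher.
; Each comparison rolls its own random index, so the odds are not a single even pick.
; The result sets the character's State and Weapon child actor class, then the pickup destroys itself.
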(event `self.Mesh.OnComponentBeginOverlap`
  (params (OverlappedComponent :type "PrimitiveComponent Object Reference") (OtherActor :type "Actor Object Reference") (OtherComp :type "PrimitiveComponent Object Reference") (OtherBodyIndex :type Integer) (bFromSweep :type Boolean) (SweepResult :type "HitResult Structure (by ref)"))
  (bind _asbp_my_character (cast `/Game/MyProj1120/GameFramework/BP_MyCharacter` OtherActor))
  (set `self.As BP My Character` _asbp_my_character)
  (bind _outrownames (`DataTableFunctionLibrary.GetDataTableRowNames` "/Game/MyProj1120/Weapon/SelfPickup/DT_Weapon.DT_Weapon"))
  (bind _output (`|GetArrayItem` _outrownames (`KismetMathLibrary.RandomIntegerInRange` 0 2)))
  (if (== _output "Pistol")
    (bind _as_bp_my_character (`self.As BP My Character`)
      (:`then`
        (set `MyCharacter.State` "Pistol" _as_bp_my_character)
        (`ChildActorComponent.SetChildActorClass` (`MyCharacter.Weapon` _as_bp_my_character) "/Game/MyProj1120/Weapon/BP_AutoPistol.BP_AutoPistol_C")
        (`self.K2_DestroyActor`))
      (:`else`))
    (elif (== _output "Rifle")
      (bind _as_bp_my_character_2 (`self.As BP My Character`)
        (:`then`
          (set `MyCharacter.State` "Rifle" _as_bp_my_character_2)
          (`ChildActorComponent.SetChildActorClass` (`MyCharacter.Weapon` _as_bp_my_character_2) "/Game/MyProj1120/Weapon/BP_AutoRifle.BP_AutoRifle_C")
          (`self.K2_DestroyActor`))
        (:`else`))
      (else
        (bind _as_bp_my_character_3 (`self.As BP My Character`)
          (:`then`
            (set `MyCharacter.State` "Launcher" _as_bp_my_character_3)
            (`ChildActorComponent.SetChildActorClass` (`MyCharacter.Weapon` _as_bp_my_character_3) "/Game/MyProj1120/Weapon/BP_AutoLauncher.BP_AutoLauncher_C")
            (`self.K2_DestroyActor`))
          (:`else`))))))

(fn `UserConstructionScript`)